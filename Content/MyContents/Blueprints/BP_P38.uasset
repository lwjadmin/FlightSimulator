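; BP_P38 is a player-controlled P-38 aircraft pawn that flies forward on its own and fires missiles from an arrow component.
; Tick spins the propellers from an RPM value and adds forward movement only when both are running.
; Roll, pitch and yaw axes apply scaled local rotations, while holding boost drives a timeline that raises the FloatingPawnMovement max speed and reverses it on release.
; Fire spawns BP_Missle, and key 2 spawns BP_TraceMissle.
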(event `self.ReceiveBeginPlay`
  (set `self.P38MaxSpeed` (`MovementComponent.GetMaxSpeed` (`self.FloatingPawnMovement`))))

(event `self.ReceiveTick`
  (params (DeltaSeconds :type "Float (single-precision)"))
  (`|ExecutionSequence`
    (:`then_0`
      (if (`self.bRightPropellerIsRunning`)
        (`SceneComponent.K2_AddLocalRotation` (`self.RightPropeller`) (`KismetMathLibrary.MakeRotator` (* (`GameplayStatics.GetWorldDeltaSeconds`) 6.0 (`self.PropellerRPM`))) false false)
        (if (`self.bLeftPropellerIsRunning`)
          (`SceneComponent.K2_AddLocalRotation` (`self.LeftPropeller`) (`KismetMathLibrary.MakeRotator` (* (`GameplayStatics.GetWorldDeltaSeconds`) 6.0 (`self.PropellerRPM`))) false false)
          (`self.AddMovementInput` (`self.GetActorForwardVector`)))))
    (:`then_1`
      (if (`self.bBoostPressed`)
        (bind (_direction `_새_트랙_0`) (`Timeline|타임라인_0` :!label _label)
          (:`Update`
            (set `FloatingPawnMovement.MaxSpeed` (+ (* `_새_트랙_0` (`self.P38MaxSpeed`) 3.0) (`self.P38MaxSpeed`)) (`self.FloatingPawnMovement`))))
        (else
          (goto _label :!via `Reverse`))))))

(event `InputAction|Boost`
  (params (Key :type "Key Structure"))
  (:`Pressed`
    (set `self.bBoostPressed` true))
  (:`Released`
    (set `self.bBoostPressed` false)))

(event `InputAxis|Roll`
  (params (AxisValue :type "Float (single-precision)"))
  (`self.K2_AddActorLocalRotation` (`KismetMathLibrary.MakeRotator` (* (`KismetMathLibrary.FClamp` AxisValue -1.0) (`self.P38RotationSpeed`) (`GameplayStatics.GetWorldDeltaSeconds`) 0.75))))

(event `InputAxis|Pitch`
  (params (AxisValue :type "Float (single-precision)"))
  (`self.K2_AddActorLocalRotation` (`KismetMathLibrary.MakeRotator` 0.0 (* (`KismetMathLibrary.FClamp` AxisValue -1.0) (`self.P38RotationSpeed`) (`GameplayStatics.GetWorldDeltaSeconds`) 1.0))))

(event `InputAxis|Yaw`
  (params (AxisValue :type "Float (single-precision)"))
  (`self.K2_AddActorLocalRotation` (`KismetMathLibrary.MakeRotator` 0.0 0.0 (* (`KismetMathLibrary.FClamp` AxisValue -1.0) (`self.P38RotationSpeed`) (`GameplayStatics.GetWorldDeltaSeconds`) 0.3))))

(event `InputAction|Fire`
  (params (Key :type "Key Structure"))
  (:`Pressed`
    (`|SpawnActorFromClass` "/Game/MyContents/Blueprints/BP_Missle.BP_Missle_C" (`SceneComponent.K2_GetComponentToWorld` (`self.Arrow`)) "AlwaysSpawn" "OverrideRootScale" null null)))

(event `Key|Two`
  (params (Key :type "Key Structure"))
  (:`Pressed`
    (`|SpawnActorFromClass` "/Game/MyContents/Blueprints/BP_TraceMissle.BP_TraceMissle_C" (`SceneComponent.K2_GetComponentToWorld` (`self.Arrow`)) "AlwaysSpawn" "OverrideRootScale" null null)))

(fn `UserConstructionScript`)