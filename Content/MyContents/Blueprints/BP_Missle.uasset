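; BP_Missle is a missile actor that explodes on overlap or after a timed fuse.
; A Delay on Tick acts as a ten-second lifetime, while overlap with anything other than a BP_P38, presumably the launching plane, detonates it immediately.
; Both paths call KABoom, which spawns explosion and smoke emitters, plays a sound at the missile's location and destroys the actor.
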(event `self.ReceiveTick`
  (params (DeltaSeconds :type "Float (single-precision)"))
  (`KismetSystemLibrary.Delay` 10.0)
  (`self.KA_Boom` :!label _label))

(event `self.ReceiveActorBeginOverlap`
  (params (OtherActor :type "Actor Object Reference"))
  (cast `/Game/MyContents/Blueprints/BP_P38` OtherActor
    (:`CastFailed`
      (goto _label))))

(fn `KA_Boom`
  (`GameplayStatics.SpawnEmitterAtLocation` "/Game/StarterContent/Particles/P_Explosion.P_Explosion" (`self.K2_GetActorLocation`))
  (`GameplayStatics.SpawnEmitterAtLocation` "/Game/StarterContent/Particles/P_Smoke.P_Smoke" (`self.K2_GetActorLocation`))
  (`GameplayStatics.PlaySoundAtLocation` "/Game/StarterContent/Audio/Explosion_Cue.Explosion_Cue" (`self.K2_GetActorLocation`) (struct) 1.0 1.0 0.0 null null null)
  (`self.K2_DestroyActor`))

(fn `UserConstructionScript`)